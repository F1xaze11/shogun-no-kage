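; BP_ronin is the Ronin character, which aggroes on the old samurai when it comes within range.
; When an actor begins overlapping its AggroRange component, it checks for BP_old_samurai and passes it to its AIC_Ronin controller through SetAttackTarget.
; The Blueprint has no end-overlap handling, and its BeginPlay and ActorBeginOverlap events are disabled placeholders.
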(event `self.AggroRange.OnComponentBeginOverlap`
  (params (OverlappedComponent :type "PrimitiveComponent Object Reference") (OtherActor :type "Actor Object Reference") (OtherComp :type "PrimitiveComponent Object Reference") (OtherBodyIndex :type Integer) (bFromSweep :type Boolean) (SweepResult :type "HitResult Structure (by ref)"))
  (bind _asbp_old_samurai (cast `/Game/Blueprints/Characters/Old_samurai/BP_old_samurai` OtherActor))
  (bind _asaic_ronin (cast `/Game/Blueprints/AI/AIC_Ronin` (`AIBlueprintHelperLibrary.GetAIController` self)))
  (`/Game/Blueprints/AI/AIC_Ronin.Set Attack Target` _asaic_ronin _asbp_old_samurai))

(fn `UserConstructionScript`
  (`parent.UserConstructionScript`))