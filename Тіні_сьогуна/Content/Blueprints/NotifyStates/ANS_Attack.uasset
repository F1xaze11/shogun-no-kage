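; Paper2D animation notify state that marks the attack window by toggling a character's melee hitbox collision.
; OnNotifyBegin enables the hitbox and OnNotifyEnd disables it, reaching the old samurai Blueprint through a cast on the owning instance's Paper character.
; A duplicate pair of graphs, OnNotifyBegin1 and OnNotifyEnd1, repeats the same logic for the ronin through its own class-specific cast.
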(fn `OnNotifyBegin`
  (params (OwningInstance :type "PaperZDAnimInstance Object Reference"))
  (bind _asbp_action_char_old_samurai (cast `/Game/Blueprints/Characters/BP_ActionChar_old_samurai` (`PaperZDAnimInstance.GetPaperCharacter` OwningInstance)))
  (`/Game/Blueprints/Characters/BP_ActionChar_old_samurai.SetHitboxCollision` _asbp_action_char_old_samurai true))

(fn `OnNotifyBegin1`
  (params (OwningInstance :type "PaperZDAnimInstance Object Reference"))
  (bind _asbp_action_char_ronin (cast `/Game/Blueprints/Characters/BP_ActionChar_ronin` (`PaperZDAnimInstance.GetPaperCharacter` OwningInstance)))
  (`/Game/Blueprints/Characters/BP_ActionChar_ronin.SetHitboxCollision` _asbp_action_char_ronin true))

(fn `OnNotifyEnd`
  (params (OwningInstance :type "PaperZDAnimInstance Object Reference"))
  (bind _asbp_action_char_old_samurai (cast `/Game/Blueprints/Characters/BP_ActionChar_old_samurai` (`PaperZDAnimInstance.GetPaperCharacter` OwningInstance)))
  (`/Game/Blueprints/Characters/BP_ActionChar_old_samurai.SetHitboxCollision` _asbp_action_char_old_samurai false))

(fn `OnNotifyEnd1`
  (params (OwningInstance :type "PaperZDAnimInstance Object Reference"))
  (bind _asbp_action_char_ronin (cast `/Game/Blueprints/Characters/BP_ActionChar_ronin` (`PaperZDAnimInstance.GetPaperCharacter` OwningInstance)))
  (`/Game/Blueprints/Characters/BP_ActionChar_ronin.SetHitboxCollision` _asbp_action_char_ronin false))