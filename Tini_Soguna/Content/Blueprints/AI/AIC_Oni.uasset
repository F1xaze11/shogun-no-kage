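; AI controller for the Oni enemy that runs the shared enemy behavior tree and blackboard.
; On possess it binds to the Oni's stun changes and mirrors them to the blackboard, while SetAttackTarget stores the target there and locally.
; Each tick it faces the target along the world X axis only, or holds its current forward facing when it has no target or cannot act.
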(event `self.ReceiveBeginPlay`
  (`self.UseBlackboard` "/Game/Blueprints/AI/BB_Enemy.BB_Enemy")
  (`self.RunBehaviorTree` "/Game/Blueprints/AI/BT_Enemy.BT_Enemy"))

(event `self.ReceiveTick`
  (params (DeltaSeconds :type "Float (single-precision)"))
  (`self.SetFocusDirection`))

(event `self.ReceivePossess`
  (params (PossessedPawn :type "Pawn Object Reference"))
  (bind _asbp_oni (cast `/Game/Blueprints/Characters/Oni/BP_Oni` PossessedPawn))
  (set `self.Action Char` _asbp_oni)
  (add `/Game/Blueprints/Characters/BP_ActionChar_Oni.StunStateChanged` (`self.Action Char`) (delegate `OnStunStateChanged`)))

(event `OnStunStateChanged`
  (params (IsStunned :type Boolean))
  (`BlackboardComponent.SetValueAsBool` (`self.Blackboard`) (`self.Is Stunned Key`) IsStunned))

(fn `Set Attack Target`
  (params (`Attack Target` :type "/Game/Blueprints/Characters/Old_samurai/BP_old_samurai Object Reference"))
  (`BlackboardComponent.SetValueAsObject` (`self.Blackboard`) (`self.Attack Target Key`) (`local.Attack Target`))
  (set `self.Attack Target` (`local.Attack Target`)))

(fn `SetFocusDirection`
  (bind _action_char (`self.Action Char`))
  (bind _returnvalue_x (`KismetMathLibrary.BreakVector` (`KismetMathLibrary.GetForwardVector` (`KismetMathLibrary.FindLookAtRotation` (`self.K2_GetActorLocation` (`self.Action Char`)) (`self.K2_GetActorLocation` (`self.Attack Target`))))))
  (`/Engine/EditorBlueprintResources/StandardMacros.IsValid` (`self.Attack Target`)
    (:`Is Valid`
      (if (`/Game/Blueprints/Characters/BP_ActionChar_Oni.Can Act` (`self.Action Char`))
        (`self.K2_SetFocalPoint` (+ (`self.K2_GetActorLocation` (`self.Action Char`)) (`KismetMathLibrary.MakeVector` _returnvalue_x)))
        (else
          (`self.K2_SetFocalPoint` (+ (`self.K2_GetActorLocation` _action_char) (`self.GetActorForwardVector` _action_char)) :!label _label))))
    (:`Is Not Valid`
      (goto _label))))

(fn `UserConstructionScript`)